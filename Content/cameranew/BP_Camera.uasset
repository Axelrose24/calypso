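; BP_Camera is a shared camera that follows all actors tagged "player", fading in and becoming the view target at BeginPlay.
; Each tick it moves to the players' average location and scales spring arm length with the farthest player's distance, within clamped limits.
; A BPISwitch event toggles a steeper top-down mode with fixed arm length.
; It also registers itself with the game mode through an interface call.
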(event EventBeginPlay
  (CameraFades|StartCameraFade (Game|GetPlayerCameraManager 0) 2.0 0.0 1.0 "(R=0.000000,G=0.000000,B=0.000000,A=1.000000)" false false)
  (Utilities|FlowControl|Delay 0.2)
  (Game|Player|SetViewTargetwithBlend (Game|GetPlayerController 0) self 0.1 "VTBlend_Linear" 0.0 false)
  (bind _outactors (Actor|GetAllActorswithTag "player"))
  (Variables|Default|SetPlayers _outactors)
  (Class|BPICameraSwitch|BPIRegister(Message) (Game|GetGameMode) self))

(event EventTick
  (params (DeltaSeconds :type Float%20%28single-precision%29))
  (Variables|Default|SetFurthestDistacne 0.0)
  (bind _returnvalue (Class|GameplayStatics|GetActorArrayAverageLocation (Variables|Default|GetPlayers)))
  (Transformation|SetWorldLocation (Variables|Transformation|GetRootComponent) _returnvalue false true)
  (if (Variables|Default|GetIsTopDown)
    (Variables|/Script/Engine.SpringArmComponent|SetTargetArmLength (Variables|Default|GetSpringArm) (Variables|Default|GetTopDownLength))
    (Transformation|SetWorldRotation (Variables|Default|GetSpringArm) "-70.000000,0.000000,0.000000" false false)
    (else
      (for _array_element (Variables|Default|GetPlayers)
        (if (> (Transformation|GetDistanceTo _array_element) (Variables|Default|GetFurthestDistacne))
          (Variables|Default|SetFurthestDistacne (Transformation|GetDistanceTo _array_element))))
      (Variables|/Script/Engine.SpringArmComponent|SetTargetArmLength (Variables|Default|GetSpringArm) (Math|Float|Clamp(Float) (* (Variables|Default|GetFurthestDistacne) 1.3) 7e+02 (Variables|Default|GetTopDownLength)))
      (Transformation|SetWorldRotation (Variables|Default|GetSpringArm) "-40.000000,0.000000,0.000000" false false))))

(event EventBPISwitch
  (Variables|Default|SetIsTopDown (not (Variables|Default|GetIsTopDown))))

(fn ConstructionScript)

(fn BPIGetCamera
  (return 0))