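; AI spawn actor that repeatedly seeks the nearest nearby actor tagged "Interact", treated as a player, and glides toward it.
; BeginPlay calls CreatePlayer, then loops on a short delay, sphere-tracing around itself to fill PlayersInRange, which is never cleared.
; The closest entry drives MoveComponentTo on the root, bypassing navigation, with duration scaled by distance for roughly constant speed.
; Trace drawing and printed durations serve as debug output.
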(event Custom|GetLocationOfNearestPlayer
  (bind _rootcomponent (Variables|Transformation|GetRootComponent))
  (bind _returnvalue (Transformation|GetWorldLocation _rootcomponent))
  (bind _outhits (Collision|MultiSphereTraceByChannel _returnvalue _returnvalue 1e+03 "TraceTypeQuery1" false 0 "ForDuration"))
  (bind (_array_element _array_index) (Utilities|Array|ForEachLoopwithBreak _outhits)
    (:LoopBody
      (if (Actor|ActorHasTag (.HitActor (Collision|BreakHitResult _array_element)) "Interact")
        (Utilities|Array|SetArrayElem (Variables|Default|GetPlayersInRange) _array_index (.HitActor (Collision|BreakHitResult _array_element)) true)))
    (:Completed
      (Variables|Default|SetNearestActorLocation (.ReturnValue (Actor|FindNearestActor (Transformation|GetWorldLocation (Variables|Transformation|GetRootComponent)) (Variables|Default|GetPlayersInRange)))))))

(event Custom|MoveTo
  (bind _nearestactorlocation (Variables|Default|GetNearestActorLocation))
  (bind _returnvalue (Transformation|GetDistanceTo _nearestactorlocation))
  (bind _returnvalue_2 (/ _returnvalue 1e+02))
  (Development|PrintString (Utilities|String|ToString(Float) _returnvalue_2))
  (Components|MoveComponentTo (Variables|Transformation|GetRootComponent) (Transformation|GetActorLocation (Variables|Default|GetNearestActorLocation)) "0, 0, 0" false false _returnvalue_2 false))

(event EventBeginPlay
  (Class|GameplayStatics|CreatePlayer 0)
  (CallFunction|GetLocationOfNearestPlayer :!label _label)
  (CallFunction|Moveto)
  (Utilities|FlowControl|Delay 0.4)
  (goto _label))

(fn ConstructionScript)