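; BP_EnemySpawnPlatform is a platform actor that spawns a fixed batch of BP_AISpawn actors when play begins.
; BeginPlay passes the batch size to the SpawnEnemy event, which loops through a one-second Delay until the Spawned counter reaches it.
; Each actor spawns slightly above the platform's location, with collision handling set to always spawn.
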(event Custom|SpawnEnemy
  (params (Number :type Integer))
  (bind _returnvalue (Transformation|GetActorTransform))
  (if (not (>= (Variables|Default|GetSpawned) Number)) :!label _label
    (Game|SpawnActorfromClass "/Game/EnemyAI/BP_AISpawn.BP_AISpawn_C" (Math|Transform|MakeTransform (Math|Vector|MakeVector (.x (.location _returnvalue)) (.y (.location _returnvalue)) (+ (.z (.location _returnvalue)) 1e+01)) "0, 0, 0" "1.000000,1.000000,1.000000") "AlwaysSpawn" "MultiplyWithRoot" 0 0)
    (Math|Integer|IncrementInt (Variables|Default|GetSpawned)
      (:%20%20
        (Utilities|FlowControl|Delay 1.0)
        (goto _label)))))

(event EventBeginPlay
  (CallFunction|SpawnEnemy 10))

(fn ConstructionScript)