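; Timer button puzzle piece that messages a connected object when an actor tagged "interact" overlaps its box, then again when the timer expires.
; Each overlap restarts the timer and a timeline-driven progress bar widget, with play rate scaled to the timer length.
; A DoOnce limits the power message to the first press until expiry hides the bar and resets it.
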(event OnComponentBeginOverlap(Box)
  (params (OverlappedComponent :type Primitive%20Component%20Object%20Reference) (OtherActor :type Actor%20Object%20Reference) (OtherComp :type Primitive%20Component%20Object%20Reference) (OtherBodyIndex :type Integer) (bFromSweep :type Boolean) (SweepResult :type Hit%20Result%20Structure%20%28by%20ref%29))
  (if (Actor|ActorHasTag OtherActor "interact")
    (Utilities|Time|SetTimerbyEvent (delegate Custom|Timer%20Expired) (Variables|Default|GetTimerLength))
    (Utilities|FlowControl|Sequence
      (:then_0
        (Utilities|FlowControl|DoOnce false
          (:Completed
            (Class|BPIPuzzleMechanics|BPIPower(Message) (Variables|Default|GetConnectedObject) self))))
      (:then_1
        _))
    (Rendering|SetVisibility (Variables|Default|GetProgressBar) true false)
    (bind _intime (Timeline|DoProgressBar PlayFromStart)
      (:Update
        (Class|BPIPuzzleMechanics|BPISetProgressBarTime(Message) (UserInterface|GetUserWidgetObject (Variables|Default|GetProgressBar)) _intime)))))

(event Custom|Timer%20Expired
  (Class|BPIPuzzleMechanics|BPIPower(Message) (Variables|Default|GetConnectedObject) self)
  (Rendering|SetVisibility (Variables|Default|GetProgressBar) false false)
  (Utilities|FlowControl|DoOnce false) ; enters at Reset
)

(event EventBeginPlay
  (Components|Timeline|SetPlayRate (Variables|Default|GetDoProgressBar) (/ 1.0 (Variables|Default|GetTimerLength))))

(fn ConstructionScript)

(fn BPIComponenttoAttachto
  (return 0))