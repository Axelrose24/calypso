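; BP_TimerActivate is a puzzle mechanic that activates its connected objects on a repeating timer.
; BeginPlay starts a looping timer at TimerSeconds, and each tick sends BPIActivateMessage to every entry in ConnectedObjects.
; A FlipFlop inside the loop picks Forward or Backward, so direction alternates per message rather than per tick.
; The construction script displays the interval on a TextRender.
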(event Custom|Flip
  (for _array_element (Variables|Default|GetConnected%20Objects)
    (bind _isa (Utilities|FlowControl|FlipFlop)
      (:A
        _)
      (:B
        _))
    (Class|BPIPuzzleMechanics|BPIActivate(Message) _array_element (select _isa "Forward" "Backward"))))

(event EventBeginPlay
  (Utilities|Time|SetTimerbyEvent (delegate Custom|Flip) (Variables|Default|GetTimer%20%28Seconds%29) true))

(fn ConstructionScript
  (Rendering|Components|TextRender|SetText (Variables|Default|GetTextRender) (Utilities|Text|ToText(Float) (Variables|Default|GetTimer%20%28Seconds%29) "HalfToEven")))

(fn BPIComponenttoAttachto
  (return 0))