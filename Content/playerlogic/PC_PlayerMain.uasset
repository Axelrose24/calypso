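; Player controller for local multiplayer that registers players, spawns their character and routes their input to it.
; Controller 0 auto-registers; others register by any key on the selection level, with state stored in the GameInstance by controller ID.
; Initialise applies the keyboard/mouse or gamepad mapping context, then async-loads, spawns and possesses the character.
; Aiming rotates the mesh via cursor timer or stick; right-click fires a class ability behind a cooldown.
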(event Custom|Initialise
  (Utilities|IsValid (Variables|Default|GetowningCharacter)
    (:Is%20Valid
      (Development|PrintString "has character"))
    (:Is%20Not%20Valid
      (CallFunction|SetUpPlayerInfo)
      (Input|AddMappingContext (PlayerController|LocalPlayerSubsystems|GetEnhancedInputLocalPlayerSubsystem) (Utilities|Select :Index (.controlscheme (CallFunction|GetPlayerInfo)) :NewEnumerator0 "/Game/playerlogic/input/IAC_PlayerMainKeyboard.IAC_PlayerMainKeyboard" :NewEnumerator1 "/Game/playerlogic/input/IAC_PlayerMainController.IAC_PlayerMainController") 0 "(bIgnoreAllPressedKeysUntilRelease=True,bForceImmediately=False,bNotifyUserSettings=False)")
      (if (Variables|Default|Getregistered)
        (bind _class (Utilities|AsyncLoadClassAsset (Variables|Default|GetAsset%20Class))
          (:Completed
            (bind _ascharacter (Utilities|Casting|CastToCharacterClass _class))
            (bind _returnvalue (Actor|GetActorOfClass "/Script/Engine.PlayerStart"))
            (bind _returnvalue_2 (Game|SpawnActorfromClass _ascharacter (Math|Transform|MakeTransform (Transformation|GetActorLocation _returnvalue) "0, 0, 0" "1.000000,1.000000,1.000000") "Undefined" "MultiplyWithRoot" 0 0))
            (bind _output_get (Variables|Default|SetowningCharacter _returnvalue_2))
            (Pawn|Possess _output_get)
            (switch Utilities|FlowControl|Switch|SwitchonENUM_ControlScheme (.controlscheme (CallFunction|GetPlayerInfo))
              (:NewEnumerator0
                (Utilities|Time|SetTimerbyFunctionName 0 "lookAtMouse" 0.01 true true)
                (Variables|Default|SetbShowMouseCursor true)))))))))

(event Custom|debugchecks
  ;[1 0 0 0.5] Debug Tools
  (Utilities|IsValid (Variables|Default|GetowningCharacter)
    (:Is%20Valid
      (|hascharacter))
    (:Is%20Not%20Valid
      (|nocharactererrorwarning))))

(event Custom|DeregisterPlayer
  ;[1 0 0 0.5] Deregister a player
  (bind _structout (Utilities|Struct|SetmembersinSTRUCT_PlayerInfo (Variables|Default|GetplayerInfo) false))
  (CallFunction|UpdatePlayerInfo _structout))

(event Custom|CreatePlayerIdentifiers)

(event Input|EnhancedActionEvents|EnhancedInputActionIA_AttackNew
  (params (ActionValue :type Boolean) (ElapsedSeconds :type Float%20%28double-precision%29) (TriggeredSeconds :type Float%20%28double-precision%29) (InputAction :type Input%20Action%20Object%20Reference :default "/Game/playerlogic/input/IA_AttackNew.IA_AttackNew"))
  (Class|BPIPlayer|BPIAttack(Message) (Variables|Default|GetowningCharacter) (.controlscheme (CallFunction|GetPlayerInfo))))

(event Input|EnhancedActionEvents|EnhancedInputActionIA_MoveNew
  (params (ActionValue :type Vector%202D%20Structure) (ElapsedSeconds :type Float%20%28double-precision%29) (TriggeredSeconds :type Float%20%28double-precision%29) (InputAction :type Input%20Action%20Object%20Reference :default "/Game/playerlogic/input/IA_MoveNew.IA_MoveNew"))
  (Pawn|Input|AddMovementInput (Variables|Default|GetowningCharacter) (Transformation|GetActorForwardVector (Variables|Default|GetowningCharacter)) (.x ActionValue) false)
  (Pawn|Input|AddMovementInput (Variables|Default|GetowningCharacter) (Transformation|GetActorRightVector (Variables|Default|GetowningCharacter)) (.y ActionValue) false))

(event Input|EnhancedActionEvents|EnhancedInputActionIA_AimControllerNew
  (params (ActionValue :type Vector%202D%20Structure) (ElapsedSeconds :type Float%20%28double-precision%29) (TriggeredSeconds :type Float%20%28double-precision%29) (InputAction :type Input%20Action%20Object%20Reference :default "/Game/playerlogic/input/IA_AimControllerNew.IA_AimControllerNew"))
  (Transformation|SetWorldRotation (Variables|/Script/Engine.Character|GetMesh (Variables|Default|GetowningCharacter)) (Math|Conversions|RotationFromXVector (Math|Vector|MakeVector (.y ActionValue) (.x ActionValue) 0.0)) false false))

(event EventBeginPlay
  ;[1 0 0 0.5] On begin play, if the player controller is 0, auto register it. This is so the keyboard "main player" always has a player controller connected to its local player.
  (if (== (Class|GameplayStatics|GetPlayerControllerID self) 0)
    (CallFunction|RegisterPlayer)))

(event Input|KeyboardEvents|SpaceBar
  (params (Key :type Key%20Structure :default "None"))
  (:Pressed
    (Character|Jump (Variables|Default|GetowningCharacter))))

(event Input|GamepadEvents|GamepadFaceButtonRight
  (params (Key :type Key%20Structure :default "None"))
  (:Pressed
    (Character|Jump (Variables|Default|GetowningCharacter))))

(event Input|MouseEvents|RightMouseButton
  (params (Key :type Key%20Structure :default "None"))
  (:Pressed
    (Utilities|Cooldown 5.0
      (:immediate
        (switch Utilities|FlowControl|Switch|SwitchonENUM_SecondaryAttack (.membervar (CallFunction|GetPlayerClass))
          (:NewEnumerator0
            (Default|AbilitySlam (Variables|Default|GetBPAC_Abilities) (Variables|Default|GetowningCharacter)))
          (:NewEnumerator1
            (Default|AbilityPunch (Variables|Default|GetBPAC_Abilities) (Variables|Default|GetowningCharacter))))))))

(event Input|KeyboardEvents|AnyKey
  (params (Key :type Key%20Structure :default "None"))
  (:Pressed
    (bind _returnvalue (Game|GetCurrentLevelName true))
    (if (Utilities|Enum|Equal(Enum) _returnvalue "lv_selectioncool")
      (Class|BPISelectionInterface|BPIAddUser(Message) (Game|GetGameMode) self)
      (CallFunction|RegisterPlayer))))

(fn ConstructionScript)

(fn GetPlayerInfo
  (bind _info (Class|BPISelectionInterface|BPIGetPlayerInfo(Message) (Game|GetGameInstance) (Class|GameplayStatics|GetPlayerControllerID self)))
  (return _info))

(fn SetUpPlayerInfo
  (bind _output_get (Variables|Default|SetplayerInfo (CallFunction|GetPlayerInfo)))
  (Variables|Default|Setregistered (.registered _output_get))
  (return))

(fn LookatMouse
  (if (Variables|Default|Getregistered)
    (Transformation|SetRelativeRotation (Variables|/Script/Engine.Character|GetMesh (Variables|Default|GetowningCharacter)) (Math|Rotator|MakeRotator 0.0 0.0 (+ 9e+01 (.yaw (Math|Rotator|FindLookatRotation (.location (.HitResult (Game|Player|GetHitResultUnderCursorbyChannel "TraceTypeQuery1" true))) (Transformation|GetActorLocation (Pawn|GetControlledPawn)))))) false false)))

(fn UpdatePlayerInfo
  (params (In :type STRUCT%20Player%20Info%20Structure))
  (Class|BPISelectionInterface|BPIUpdatePlayerInfo(Message) (Game|GetGameInstance) (Class|GameplayStatics|GetPlayerControllerID self) In))

(fn RegisterPlayer
  (Variables|Default|Setregistered true)
  (bind _structout (Utilities|Struct|SetmembersinSTRUCT_PlayerInfo (CallFunction|GetPlayerInfo) true))
  (CallFunction|UpdatePlayerInfo _structout))

(fn GetPlayerClass
  (bind _class (Class|BPISelectionInterface|BPIGetPlayerChosenClass(Message) (Game|GetGameInstance) (Class|GameplayStatics|GetPlayerControllerID self)))
  (return _class))