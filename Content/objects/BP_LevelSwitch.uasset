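; BP_LevelSwitch is a trigger box that moves the game to a configured level once all players have entered it.
; It takes the player count from the GameState at BeginPlay, then freezes and counts each overlapping character tagged "player".
; When the count reaches that number, it fades player 0's camera out, waits briefly and opens the level; until then it prints the progress for debugging.
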(event OnComponentBeginOverlap(Box)
  (params (OverlappedComponent :type Primitive%20Component%20Object%20Reference) (OtherActor :type Actor%20Object%20Reference) (OtherComp :type Primitive%20Component%20Object%20Reference) (OtherBodyIndex :type Integer) (bFromSweep :type Boolean) (SweepResult :type Hit%20Result%20Structure%20%28by%20ref%29))
  (if (Actor|ActorHasTag OtherActor "player")
    (bind _ascharacter (Utilities|Casting|CastToCharacter OtherActor))
    (Pawn|Components|CharacterMovement|DisableMovement (Variables|/Script/Engine.Character|GetCharacterMovement _ascharacter))
    (bind _result (Math|Integer|IncrementInt (Variables|Default|Getcurrent))
      (:%20%20
        (if (>= _result (Variables|Default|Getrequired))
          (CameraFades|StartCameraFade :self (Variables|/Script/Engine.PlayerController|GetPlayerCameraManager (Game|GetPlayerController 0)) :FromAlpha 0.0 :ToAlpha 1.0 :Duration 1.5 :bHoldWhenFinished true)
          (Utilities|FlowControl|Delay 2.5)
          (Game|OpenLevel(byName) (Variables|Default|GetOpen%20Level))
          (else
            (|debug:notenough)))))))

(event EventBeginPlay
  (Variables|Default|Setrequired (Utilities|Array|Length (Variables|/Script/Engine.GameStateBase|GetPlayerArray (Game|GetGameState)))))

(fn ConstructionScript)